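; BP_ClimbingPlayerController is the player controller for the climbing character, turning Enhanced Input actions into movement and camera commands.
; On BeginPlay it adds the climbing input mapping context and caches the controlled pawn as a BP_ClimbingCharacter.
; Camera rotate left, rotate right, reset and move-to-location actions forward straight to that character, which implements the behavior.
; The move command passes the controller itself to the character.
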(event Input|EnhancedActionEvents|EnhancedInputActionIA_RotateCameraLeft
  (params (ActionValue :type Boolean) (ElapsedSeconds :type Float%20%28double-precision%29) (TriggeredSeconds :type Float%20%28double-precision%29) (InputAction :type Input%20Action%20Object%20Reference :default "/Game/Inputs/InputActions/IA_RotateCameraLeft.IA_RotateCameraLeft"))
  (Class|ClimbingCharacter|RotateCameraLeft (Variables|Default|GetClimbingCharacterRef)))

(event Input|EnhancedActionEvents|EnhancedInputActionIA_RotateCameraRight
  (params (ActionValue :type Boolean) (ElapsedSeconds :type Float%20%28double-precision%29) (TriggeredSeconds :type Float%20%28double-precision%29) (InputAction :type Input%20Action%20Object%20Reference :default "/Game/Inputs/InputActions/IA_RotateCameraRight.IA_RotateCameraRight"))
  (Class|ClimbingCharacter|RotateCameraRight (Variables|Default|GetClimbingCharacterRef)))

(event Input|EnhancedActionEvents|EnhancedInputActionIA_MoveToLocation
  (params (ActionValue :type Boolean) (ElapsedSeconds :type Float%20%28double-precision%29) (TriggeredSeconds :type Float%20%28double-precision%29) (InputAction :type Input%20Action%20Object%20Reference :default "/Game/Inputs/InputActions/IA_MoveToLocation.IA_MoveToLocation"))
  (Default|MoveClimbingCharactertoLocation (Variables|Default|GetClimbingCharacterRef) self))

(event Input|EnhancedActionEvents|EnhancedInputActionIA_ResetCameraRotation
  (params (ActionValue :type Boolean) (ElapsedSeconds :type Float%20%28double-precision%29) (TriggeredSeconds :type Float%20%28double-precision%29) (InputAction :type Input%20Action%20Object%20Reference :default "/Game/Inputs/InputActions/IA_ResetCameraRotation.IA_ResetCameraRotation"))
  (Class|ClimbingCharacter|ResetCameraRotation (Variables|Default|GetClimbingCharacterRef)))

(event EventBeginPlay
  (Input|AddMappingContext (PlayerController|LocalPlayerSubsystems|GetEnhancedInputLocalPlayerSubsystem) "/Game/Inputs/InputMappingContexts/IMC_ClimbingCharacter.IMC_ClimbingCharacter" 0 "(bIgnoreAllPressedKeysUntilRelease=True,bForceImmediately=False,bNotifyUserSettings=False)")
  (bind _asbp_climbing_character (Utilities|Casting|CastToBP_ClimbingCharacter (Pawn|GetControlledPawn)))
  (Variables|Default|SetClimbingCharacterRef _asbp_climbing_character))

(fn ConstructionScript)